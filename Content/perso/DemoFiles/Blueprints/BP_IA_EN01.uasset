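; BP_IA_EN01 is an AI-driven actor, apparently an enemy, that starts its behavior tree when play begins.
; BeginPlay runs the Ai_spawn_bhvc tree on its AI controller, then writes player 0's current location to the "spawnLocation" blackboard key.
; Despite the key's name, it holds a one-time snapshot of the player's position, not this actor's own.
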(event `self.ReceiveBeginPlay`
  (`AIController.RunBehaviorTree` (`AIBlueprintHelperLibrary.GetAIController` self) "/Game/perso/DemoFiles/Blueprints/ai_spawn_bhvc.ai_spawn_bhvc")
  (`BlackboardComponent.SetValueAsVector` (`AIBlueprintHelperLibrary.GetBlackboard` self) "spawnLocation" (`self.K2_GetActorLocation` (`GameplayStatics.GetPlayerCharacter` 0))))

(fn `UserConstructionScript`
  (`parent.UserConstructionScript`))